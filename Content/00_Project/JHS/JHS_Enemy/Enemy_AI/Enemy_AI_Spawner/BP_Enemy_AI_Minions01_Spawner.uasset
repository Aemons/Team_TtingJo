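; Spawner actor that populates an area with BP_JHS_Enemy_Minions_01 enemies on BeginPlay.
; It spawns one minion per EnemyMinions01Array entry at a random reachable navmesh point within the Sphere radius, with random yaw.
; Each minion gets a random skeletal mesh and slot 0 material, both indices drawn up to the SkeletalMesh array's length, inclusive.
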(event EventBeginPlay
  (bind _skeletal_mesh (Variables|Enemy|GetSkeletal%20Mesh))
  (bind _returnvalue (Utilities|Array|Length _skeletal_mesh))
  (bind _returnvalue_2 (Math|Random|RandomIntegerinRange 0 _returnvalue))
  (for _array_element (Variables|Enemy|GetEnemy_Minions01_Array)
    (bind _returnvalue_3 (Game|SpawnActorfromClass "/Game/00_Project/JHS/JHS_Enemy/Enemy_Child/BP_JHS_Enemy_Minions_01.BP_JHS_Enemy_Minions_01_C" (Math|Transform|MakeTransform (.RandomLocation (AI|Navigation|GetRandomReachablePointinRadius (Transformation|GetActorLocation) (Variables|/Script/Engine.SphereComponent|GetSphereRadius (Variables|Default|GetSphere)) 0 0)) (Math|Rotator|MakeRotator 0.0 0.0 (Math|Random|RandomFloatinRange -1.8e+02 1.8e+02)) "1.000000,1.000000,1.000000") "AdjustIfPossibleButAlwaysSpawn" "MultiplyWithRoot" 0 0))
    ;[1 1 1] Enemy SkeletalMesh/Material Random Setting
    (Components|SkeletalMesh|SetSkeletalMeshAsset (Variables|/Script/Engine.Character|GetMesh _returnvalue_3) (Utilities|Array|Get(acopy) (Variables|Enemy|GetSkeletal%20Mesh) _returnvalue_2))
    (Rendering|Material|SetMaterial (Variables|/Script/Engine.Character|GetMesh _returnvalue_3) 0 (Utilities|Array|Get(acopy) (Variables|Enemy|GetSkeletal%20Material) _returnvalue_2))))

(fn ConstructionScript)